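; BP_Main is a gameplay coordinator Blueprint that sets up the HUD and handles game over.
; On BeginPlay it creates and displays the WB_UI widget, then caches the PS_PlayerState and the BP_Player pawn for player 0.
; Its GameOver event triggers the UI death display and the player's death, waits briefly, then opens the Title level.
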(event `self.ReceiveBeginPlay`
  (`|ExecutionSequence`
    (:`then_0`
      (bind _returnvalue (`|CreateWidget` "/Game/Blueprint/WB_UI.WB_UI_C"))
      (bind _output_get (set `self.UI` _returnvalue))
      (`UserWidget.AddToViewport` _output_get 0))
    (:`then_1`
      (bind _asps_player_state (cast `/Game/Blueprint/PS_PlayerState` (`GameplayStatics.GetPlayerState` 0)))
      (set `self.As PS Player State` _asps_player_state))
    (:`then_2`
      (bind _asbp_player (cast `/Game/Blueprint/BP_Player` (`GameplayStatics.GetPlayerPawn` 0)))
      (set `self.As BP Player` _asbp_player))))

(event `self.ReceiveTick`
  (params (DeltaSeconds :type "Float (single-precision)")))

(event `GameOver`
  (`/Game/Blueprint/WB_UI.YOUDIE` (`self.UI`))
  (`/Game/Blueprint/BP_Player.DIe` (`self.As BP Player`))
  (`KismetSystemLibrary.Delay` 1.0)
  (`GameplayStatics.OpenLevel` "Title"))

(fn `UserConstructionScript`)