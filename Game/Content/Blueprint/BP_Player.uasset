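; Player pawn for a 2D flipbook sprite character with four-directional movement, attack and death animations.
; On BeginPlay it adds the Enhanced Input mapping context and caches the player state.
; Move inputs add movement, swap walk/idle flipbooks and track facing, reusing the right-facing art rotated for left.
; The action input plays a directional attack flipbook, then returns to idle and calls EXP on the player state when completed.
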(event `self.ReceiveBeginPlay`
  (`|ExecutionSequence`
    (:`then_0`
      (bind _asbp_player_controler (cast `/Game/Blueprint/BP_PlayerControler` (`self.GetController`)))
      (`EnhancedInputSubsystemInterface.AddMappingContext` (pcsubsystem `EnhancedInputLocalPlayerSubsystem` _asbp_player_controler) "/Game/Blueprint/IMC_Input.IMC_Input" 0 (struct)))
    (:`then_1`
      (bind _asps_player_state (cast `/Game/Blueprint/PS_PlayerState` (`GameplayStatics.GetPlayerState` 0)))
      (set `self.As PS Player State` _asps_player_state))))

(event `EnhancedInput|/Game/Blueprint/IA_PlayerHMove`
  (params (ActionValue :type "Float (double-precision)") (ElapsedSeconds :type "Float (double-precision)") (TriggeredSeconds :type "Float (double-precision)") (InputAction :type "InputAction Object Reference" :default "/Game/Blueprint/IA_PlayerHMove.IA_PlayerHMove"))
  (bind _sprite (`self.Sprite`))
  (:`Triggered`
    (`self.AddMovementInput` (0.25 0.0 0.0) ActionValue)
    (`PaperFlipbookComponent.SetFlipbook` _sprite "/Game/Art/Warrior/PB_Player_Move_R.PB_Player_Move_R")
    (if (> ActionValue 0.0)
      (`SceneComponent.K2_SetWorldRotation` :`self` _sprite)
      (set `self.direction` 1)
      (else
        (`SceneComponent.K2_SetWorldRotation` _sprite (struct :`Yaw` -180.0) false false)
        (set `self.direction` 2))))
  (:`Completed`
    (`PaperFlipbookComponent.SetFlipbook` _sprite "/Game/Art/Warrior/PB_Player_Idle_R.PB_Player_Idle_R")))

(event `EnhancedInput|/Game/Blueprint/IA_PlayerVMove`
  (params (ActionValue :type "Float (double-precision)") (ElapsedSeconds :type "Float (double-precision)") (TriggeredSeconds :type "Float (double-precision)") (InputAction :type "InputAction Object Reference" :default "/Game/Blueprint/IA_PlayerVMove.IA_PlayerVMove"))
  (:`Triggered`
    (`self.AddMovementInput` (0.0 0.25 0.0) ActionValue)
    (if (> ActionValue 0.0)
      (`PaperFlipbookComponent.SetFlipbook` (`self.Sprite`) "/Game/Art/Warrior/PB_Player_Move_B.PB_Player_Move_B")
      (set `self.Front` false)
      (set `self.direction` 0)
      (else
        (`PaperFlipbookComponent.SetFlipbook` (`self.Sprite`) "/Game/Art/Warrior/PB_Player_Move_F.PB_Player_Move_F")
        (set `self.Front` true)
        (set `self.direction` 3))))
  (:`Completed`
    (if (`self.Front`)
      (`PaperFlipbookComponent.SetFlipbook` (`self.Sprite`) "/Game/Art/Warrior/PB_Player_Idle_F.PB_Player_Idle_F")
      (else
        (`PaperFlipbookComponent.SetFlipbook` (`self.Sprite`) "/Game/Art/Warrior/PB_Player_Idle_B.PB_Player_Idle_B")))))

(event `EnhancedInput|/Game/Blueprint/IA_PlayerAction`
  (params (ActionValue :type Boolean) (ElapsedSeconds :type "Float (double-precision)") (TriggeredSeconds :type "Float (double-precision)") (InputAction :type "InputAction Object Reference" :default "/Game/Blueprint/IA_PlayerAction.IA_PlayerAction"))
  (:`Triggered`
    (`|ExecutionSequence`
      (:`then_0`
        (if (== (`self.direction`) 0)
          (`PaperFlipbookComponent.SetFlipbook` (`self.Sprite`) "/Game/Art/Warrior/PB_Player_Attack_B.PB_Player_Attack_B")))
      (:`then_1`
        (if (== (`self.direction`) 1)
          (`PaperFlipbookComponent.SetFlipbook` (`self.Sprite`) "/Game/Art/Warrior/PB_Player_Attack_R.PB_Player_Attack_R")))
      (:`then_2`
        (if (== (`self.direction`) 2)
          (`PaperFlipbookComponent.SetFlipbook` (`self.Sprite`) "/Game/Art/Warrior/PB_Player_Attack_R.PB_Player_Attack_R")))
      (:`then_3`
        (if (== (`self.direction`) 3)
          (`PaperFlipbookComponent.SetFlipbook` (`self.Sprite`) "/Game/Art/Warrior/PB_Player_Attack_F.PB_Player_Attack_F")))))
  (:`Completed`
    (`|ExecutionSequence`
      (:`then_0`
        (if (== (`self.direction`) 0)
          (`PaperFlipbookComponent.SetFlipbook` (`self.Sprite`) "/Game/Art/Warrior/PB_Player_Idle_B.PB_Player_Idle_B")
          (`/Game/Blueprint/PS_PlayerState.EXP+` (`self.As PS Player State`))))
      (:`then_1`
        (if (== (`self.direction`) 1)
          (`PaperFlipbookComponent.SetFlipbook` (`self.Sprite`) "/Game/Art/Warrior/PB_Player_Idle_R.PB_Player_Idle_R")
          (`/Game/Blueprint/PS_PlayerState.EXP+` (`self.As PS Player State`))))
      (:`then_2`
        (if (== (`self.direction`) 2)
          (`PaperFlipbookComponent.SetFlipbook` (`self.Sprite`) "/Game/Art/Warrior/PB_Player_Idle_R.PB_Player_Idle_R")
          (`/Game/Blueprint/PS_PlayerState.EXP+` (`self.As PS Player State`))))
      (:`then_3`
        (if (== (`self.direction`) 3)
          (`PaperFlipbookComponent.SetFlipbook` (`self.Sprite`) "/Game/Art/Warrior/PB_Player_Idle_F.PB_Player_Idle_F")
          (`/Game/Blueprint/PS_PlayerState.EXP+` (`self.As PS Player State`)))))))

(event `DIe`
  (`PaperFlipbookComponent.SetFlipbook` (`self.Sprite`) "/Game/Art/Warrior/PB_Player_Die.PB_Player_Die"))

(fn `UserConstructionScript`)